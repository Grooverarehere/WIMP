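; Gate actor, a child Blueprint, that starts open and exposes OpenDoor and CloseDoor events to open and close it.
; Each event casts the SKDoorFrame skeletal mesh's anim instance to BP_Anim_Gate and sets GateState to a downward open or close state.
; BeginPlay runs the parent logic, then applies the open state; the gate's motion is left to the animation Blueprint.
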(event EventBeginPlay
  (|CallParentFunction)
  (bind _asbp_anim_gate (Utilities|Casting|CastToBP_Anim_Gate (Components|SkeletalMesh|GetAnimInstance (Variables|Default|GetSK_DoorFrame))))
  (Variables|/Game/ModularPlatforms/Animations/BP_Anim_Gate.BP_Anim_Gate_C|SetGateState _asbp_anim_gate "openDown"))

(event Collision|EventActorBeginOverlap
  (params (OtherActor :type Actor%20Object%20Reference)))

(event EventTick
  (params (DeltaSeconds :type Float%20%28single-precision%29)))

(event EventCloseDoor
  (bind _asbp_anim_gate (Utilities|Casting|CastToBP_Anim_Gate (Components|SkeletalMesh|GetAnimInstance (Variables|Default|GetSK_DoorFrame))))
  (Variables|/Game/ModularPlatforms/Animations/BP_Anim_Gate.BP_Anim_Gate_C|SetGateState _asbp_anim_gate "closeDown"))

(event EventOpenDoor
  (bind _asbp_anim_gate (Utilities|Casting|CastToBP_Anim_Gate (Components|SkeletalMesh|GetAnimInstance (Variables|Default|GetSK_DoorFrame))))
  (Variables|/Game/ModularPlatforms/Animations/BP_Anim_Gate.BP_Anim_Gate_C|SetGateState _asbp_anim_gate "openDown"))

(fn ConstructionScript)