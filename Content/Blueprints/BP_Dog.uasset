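; BP_Dog is a robot dog whose animation state reacts to overlaps.
; When BP_Marian enters WakeUpCollision while WakeUp is false, it sets ABP_RoboDog_AnimBP to "Power Off", then "Idle2" after a delay.
; When its capsule overlaps a sphere component while WakeUp is true, it clears WakeUp, returns to "Idle2" after a delay and toggles Point.
; Nothing here sets WakeUp true or reads Point.
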(event OnComponentBeginOverlap(WakeUpCollision)
  (params (OverlappedComponent :type Primitive%20Component%20Object%20Reference) (OtherActor :type Actor%20Object%20Reference) (OtherComp :type Primitive%20Component%20Object%20Reference) (OtherBodyIndex :type Integer) (bFromSweep :type Boolean) (SweepResult :type Hit%20Result%20Structure%20%28by%20ref%29))
  (Utilities|Casting|CastToBP_Marian OtherActor)
  (if (not (Variables|Default|GetWakeUp))
    (bind _asabp_robo_dog_anim_bp (Utilities|Casting|CastToABP_RoboDog_AnimBP (Components|SkeletalMesh|GetAnimInstance (Variables|Character|GetMesh))))
    (Variables|/Game/RoboDog/Robo_Dog/Blueprints/ABP_RoboDog_AnimBP.ABP_RoboDog_AnimBP_C|SetMainStateAnim _asabp_robo_dog_anim_bp "Power Off")
    (Utilities|FlowControl|Delay 1.0)
    (Variables|/Game/RoboDog/Robo_Dog/Blueprints/ABP_RoboDog_AnimBP.ABP_RoboDog_AnimBP_C|SetMainStateAnim _asabp_robo_dog_anim_bp "Idle2")))

(event OnComponentBeginOverlap(CapsuleComponent)
  (params (OverlappedComponent :type Primitive%20Component%20Object%20Reference) (OtherActor :type Actor%20Object%20Reference) (OtherComp :type Primitive%20Component%20Object%20Reference) (OtherBodyIndex :type Integer) (bFromSweep :type Boolean) (SweepResult :type Hit%20Result%20Structure%20%28by%20ref%29))
  (if (Variables|Default|GetWakeUp)
    (Utilities|Casting|CastToSphereComponent OtherComp)
    (Variables|Default|SetWakeUp false)
    (Utilities|FlowControl|Delay 0.5)
    (bind _asabp_robo_dog_anim_bp (Utilities|Casting|CastToABP_RoboDog_AnimBP (Components|SkeletalMesh|GetAnimInstance (Variables|Character|GetMesh))))
    (Variables|/Game/RoboDog/Robo_Dog/Blueprints/ABP_RoboDog_AnimBP.ABP_RoboDog_AnimBP_C|SetMainStateAnim _asabp_robo_dog_anim_bp "Idle2")
    (if (== (Variables|Default|GetPoint) 1.0)
      (Variables|Default|SetPoint 0.0)
      (else
        (Variables|Default|SetPoint 1.0)))))

(event EventBeginPlay)

(event EventTick
  (params (DeltaSeconds :type Float%20%28single-precision%29)))

(fn ConstructionScript)